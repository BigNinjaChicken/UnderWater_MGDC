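; BP_Captain supplies the Captain's dialogue content step by step, apparently for a branching conversation.
; GetNextPath serves path 0 from the Path10 struct's Log, Rsp and Evl fields, then a results path, then reports finished; a positive increase advances the path and resets the step index.
; AddToResults queues non-empty texts, which the results path pops one every third step, with "..." filling the steps between.
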(fn `AddToResults`
  (params (Results :type "Array of Text"))
  (for _array_element Results
    (if (not (`KismetTextLibrary.TextIsEmpty` _array_element))
      (`KismetArrayLibrary.Array_Add` (`self.Results`) _array_element)))
  (return))

(fn `GetNextPath`
  (params (PathStructIncrease :type Integer))
  (returns (Option :type "Array of Text") (Finished :type Boolean))
  (bind _nextpathindex (`self.NextPathIndex`))
  (if (> PathStructIncrease 0)
    (set `self.NextPathIndex` (+ 1 _nextpathindex))
    (set `self.PathStructIndex` 0))
  (switch `int` _nextpathindex
    (:`Default`
      (return _ true))
    (:`0`
      (bind _option (`self.GetPath1_0Struct`))
      (return _option false))
    (:`1`
      (bind _option_2 (`self.GetPathResultStruct`))
      (return _option_2 false))))

(fn `GetPath1_0Struct`
  (returns (Option :type "Array of Text"))
  (locals (Path1_0 :type "/Game/Game/Captain/Captain_Path1_0 Structure") (Current :type "Array of Text"))
  (bind (_log0 _rsp0 _evl0 _log1 _rsp1 _evl1) (break `/Game/Game/Captain/Captain_Path1_0` (`local.Path1_0`)))
  (bind _output_get (set `local.Current` (select `int` (`self.PathStructIndex`) :`0` _log0 :`1` _rsp0 :`2` _evl0 :`3` _log1 :`4` _rsp1 :`5` _evl1 :`6` _ :`7` _ :`8` _ :`9` _ :`10` _ :`11` _ :`12` _ :`13` _ :`14` _ :`15` _ :`16` _ :`17` _ :`18` _ :`19` _)))
  (`/Engine/EditorBlueprintResources/StandardMacros.IncrementInt` (`self.PathStructIndex`)
    (:`  `
      (return _output_get))))

(fn `GetPathResultStruct`
  (returns (Option :type "Array of Text"))
  (locals (Path1_0 :type "/Game/Game/Kid/Kid_Path1_0 Structure") (Current :type "Array of Text") (ResultLog :type "Array of Text"))
  (bind _resultlog (`local.ResultLog`))
  (bind _results (`self.Results`))
  (bind _resultlog_2 (`local.ResultLog`))
  (if (== (mod (`self.PathStructIndex`) 3) 0)
    (if (== (`KismetArrayLibrary.Array_Length` (`self.Results`)) 0)
      (`/Engine/EditorBlueprintResources/StandardMacros.IncrementInt` (`self.PathStructIndex`)
        (:`  `
          (return)))
      (else
        (`KismetArrayLibrary.Array_Clear` _resultlog_2)
        (`KismetArrayLibrary.Array_Add` _resultlog_2 (`|GetArrayItem` _results))
        (`KismetArrayLibrary.Array_Remove` _results)))
    (else
      (`KismetArrayLibrary.Array_Clear` _resultlog)
      (`KismetArrayLibrary.Array_Add` _resultlog "...")))
  (`/Engine/EditorBlueprintResources/StandardMacros.IncrementInt` (`self.PathStructIndex`)
    (:`  `
      (return (`local.ResultLog`)))))

(fn `UserConstructionScript`)