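; BP_Janitor serves the Janitor's branching sequence of Log, Rsp and Evl entries, apparently dialogue, one at a time.
; GetNextPath picks the current of three stages; a positive PathStructIncrease advances the stage and resets the entry index, with values above one choosing the top branch.
; Only the middle stage splits, into paths 2_0 and 2_1, before both rejoin at 3_0.
; Per-path getters step through struct fields using an incrementing Select index.
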(fn `Get Path 2 0Struct`
  (returns (Option :type "Array of Text"))
  (locals (Path :type "/Game/Game/Janitor/Janitor_Path2_0 Structure") (Current :type "Array of Text"))
  (bind (_log0 _rsp0 _evl0) (break `/Game/Game/Janitor/Janitor_Path2_0` (`local.Path`)))
  (bind _output_get (set `local.Current` (select `int` (`self.PathStructIndex`) :`0` _log0 :`1` _rsp0 :`2` _evl0 :`3` _ :`4` _ :`5` _ :`6` _ :`7` _ :`8` _ :`9` _ :`10` _ :`11` _ :`12` _ :`13` _ :`14` _ :`15` _ :`16` _ :`17` _ :`18` _ :`19` _)))
  (`/Engine/EditorBlueprintResources/StandardMacros.IncrementInt` (`self.PathStructIndex`)
    (:`  `
      (return _output_get))))

(fn `GetNextPath`
  (params (PathStructIncrease :type Integer))
  (returns (Option :type "Array of Text") (Finished :type Boolean))
  (bind _nextpathindex (`self.NextPathIndex`))
  (if (> PathStructIncrease 0)
    (if (> PathStructIncrease 1)
      (set `self.IsTop` true)
      (else
        (set `self.IsTop` false)))
    (set `self.NextPathIndex` (+ 1 _nextpathindex))
    (set `self.PathStructIndex` 0))
  (switch `int` _nextpathindex
    (:`Default`
      (return _ true))
    (:`0`
      (bind _option (`self.GetPath1_0Struct`))
      (return _option false))
    (:`1`
      (if (`self.IsTop`)
        (bind _option_2 (`self.Get Path 2 0Struct`))
        (return _option_2 false)
        (else
          (bind _option_3 (`self.GetPath2_1Struct`))
          (return _option_3 false))))
    (:`2`
      (if (`self.IsTop`)
        _
        (else
          _))
      (bind _option_4 (`self.GetPath3_0Struct`))
      (return _option_4 false))))

(fn `GetPath1_0Struct`
  (returns (Option :type "Array of Text"))
  (locals (Path :type "/Game/Game/Janitor/Janitor_Path1_0 Structure") (Current :type "Array of Text"))
  (bind (_log0 _rsp0 _evl0 _log1 _rsp1 _evl1 _log2 _rsp2 _evl2 _log3 _rsp3 _evl3 _log4 _rsp4 _evl4 _log5 _rsp5 _evl5 _log6 _rsp6 _evl6 _log7 _rsp7 _evl7 _log8 _rsp8 _evl8) (break `/Game/Game/Janitor/Janitor_Path1_0` (`local.Path`)))
  (bind _output_get (set `local.Current` (select `int` (`self.PathStructIndex`) :`0` _log0 :`1` _rsp0 :`2` _evl0 :`3` _log1 :`4` _rsp1 :`5` _evl1 :`6` _log2 :`7` _rsp2 :`8` _evl2 :`9` _log3 :`10` _rsp3 :`11` _evl3 :`12` _log4 :`13` _rsp4 :`14` _evl4 :`15` _log5 :`16` _rsp5 :`17` _evl5 :`18` _log6 :`19` _rsp6 :`20` _evl6 :`21` _log7 :`22` _rsp7 :`23` _evl7 :`24` _log8 :`25` _rsp8 :`26` _evl8 :`27` _ :`28` _)))
  (`/Engine/EditorBlueprintResources/StandardMacros.IncrementInt` (`self.PathStructIndex`)
    (:`  `
      (return _output_get))))

(fn `GetPath2_1Struct`
  (returns (Option :type "Array of Text"))
  (locals (Path :type "/Game/Game/Janitor/Janitor_Path2_1 Structure") (Current :type "Array of Text"))
  (bind (_log0 _rsp0 _evl0) (break `/Game/Game/Janitor/Janitor_Path2_1` (`local.Path`)))
  (bind _output_get (set `local.Current` (select `int` (`self.PathStructIndex`) :`0` _log0 :`1` _rsp0 :`2` _evl0 :`3` _ :`4` _ :`5` _ :`6` _ :`7` _ :`8` _ :`9` _ :`10` _ :`11` _ :`12` _ :`13` _ :`14` _ :`15` _ :`16` _ :`17` _ :`18` _ :`19` _)))
  (`/Engine/EditorBlueprintResources/StandardMacros.IncrementInt` (`self.PathStructIndex`)
    (:`  `
      (return _output_get))))

(fn `GetPath3_0Struct`
  (returns (Option :type "Array of Text"))
  (locals (Path :type "/Game/Game/Janitor/Janitor_Path3_0 Structure") (Current :type "Array of Text"))
  (bind (_log0 _rsp0 _evl0 _log1 _rsp1 _evl1 _log2 _rsp2 _evl2 _log3 _rsp3 _evl3 _log4 _rsp4 _evl4 _log5 _rsp5 _evl5) (break `/Game/Game/Janitor/Janitor_Path3_0` (`local.Path`)))
  (bind _output_get (set `local.Current` (select `int` (`self.PathStructIndex`) :`0` _log0 :`1` _rsp0 :`2` _evl0 :`3` _log1 :`4` _rsp1 :`5` _evl1 :`6` _log2 :`7` _rsp2 :`8` _evl2 :`9` _log3 :`10` _rsp3 :`11` _evl3 :`12` _log4 :`13` _rsp4 :`14` _evl4 :`15` _log5 :`16` _rsp5 :`17` _evl5 :`18` _ :`19` _)))
  (`/Engine/EditorBlueprintResources/StandardMacros.IncrementInt` (`self.PathStructIndex`)
    (:`  `
      (return _output_get))))

(fn `UserConstructionScript`)